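; Rotating 2x2x2 cube puzzle in which the player matches front and side silhouettes loaded from the Stage1 row of T_Answer.
; Q/A, W/S and E/D select and highlight a roll, pitch or yaw layer; J/K turn it via a timeline, composing pre-turn locations with the rotation.
; Afterwards cubes are re-indexed by position sign, and Exist/Empty tags are checked against both silhouettes, printing "Complete" on a match.
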(event EventBeginPlay
  ;[1 1 1] 正解データと初期状態をロード
  (CallFunction|LoadSideAnswer)
  (CallFunction|LoadFrontAnswer)
  (CallFunction|LoadCube)
  ;[1 1 1] 入力を有効化
  (Input|EnableInput (Game|GetPlayerController 0)))

(event Input|KeyboardEvents|E
  (params (Key :type Key%20Structure :default "None"))
  ;[1 1 1] 入力から選択箇所を変更
  (:Pressed
    (if (not (Variables|Default|GetbRotating))
      (Variables|Default|SetRotateType "NewEnumerator4")
      (bind _selectionindexarray (CallFunction|CreateSelectionIndexArray (Variables|Default|GetRotateType)))
      (bind _output_get (Variables|Default|SetSelectedIndexArray _selectionindexarray))
      (CallFunction|ChangeCubeColor _output_get))))

(event Input|KeyboardEvents|D
  (params (Key :type Key%20Structure :default "None"))
  ;[1 1 1] 入力から選択箇所を変更
  (:Pressed
    (if (not (Variables|Default|GetbRotating))
      (Variables|Default|SetRotateType "NewEnumerator5")
      (bind _selectionindexarray (CallFunction|CreateSelectionIndexArray (Variables|Default|GetRotateType)))
      (bind _output_get (Variables|Default|SetSelectedIndexArray _selectionindexarray))
      (CallFunction|ChangeCubeColor _output_get))))

(event Input|KeyboardEvents|Q
  (params (Key :type Key%20Structure :default "None"))
  ;[1 1 1] 入力から選択箇所を変更
  (:Pressed
    (if (not (Variables|Default|GetbRotating))
      (Variables|Default|SetRotateType "NewEnumerator0")
      (bind _selectionindexarray (CallFunction|CreateSelectionIndexArray (Variables|Default|GetRotateType)))
      (bind _output_get (Variables|Default|SetSelectedIndexArray _selectionindexarray))
      (CallFunction|ChangeCubeColor _output_get))))

(event Input|KeyboardEvents|A
  (params (Key :type Key%20Structure :default "None"))
  ;[1 1 1] 入力から選択箇所を変更
  (:Pressed
    (if (not (Variables|Default|GetbRotating))
      (Variables|Default|SetRotateType "NewEnumerator1")
      (bind _selectionindexarray (CallFunction|CreateSelectionIndexArray (Variables|Default|GetRotateType)))
      (bind _output_get (Variables|Default|SetSelectedIndexArray _selectionindexarray))
      (CallFunction|ChangeCubeColor _output_get))))

(event Input|KeyboardEvents|K
  (params (Key :type Key%20Structure :default "None"))
  (:Pressed
    (if (not (Variables|Default|GetbRotating))
      (Variables|Default|SetSign -1.0)
      (Utilities|FlowControl|DoOnce false :!label _label
        (:Completed
          (Variables|Default|SetbRotating true)
          (CallFunction|InitLocationArray)
          (bind _rotation (Timeline|タイムライン PlayFromStart)
            (:Update
              (for (_array_element _array_index) (Variables|Default|GetCubeArray)
                (if (Utilities|Array|ContainsItem (Variables|Default|GetSelectedIndexArray) _array_index)
                  (switch Utilities|FlowControl|Switch|SwitchonERotateType (Variables|Default|GetRotateType)
                    (:NewEnumerator0
                      (CallFunction|CubeRoll _array_element (* _rotation (Variables|Default|GetSign)) (Utilities|Array|Get(acopy) (Variables|Default|GetBeforeLocationArray) _array_index) :!label _label_2))
                    (:NewEnumerator1
                      (goto _label_2))
                    (:NewEnumerator2
                      (CallFunction|CubePitch _array_element (* _rotation (Variables|Default|GetSign)) (Utilities|Array|Get(acopy) (Variables|Default|GetBeforeLocationArray) _array_index) :!label _label_3))
                    (:NewEnumerator3
                      (goto _label_3))
                    (:NewEnumerator4
                      (CallFunction|CubeYaw _array_element (* _rotation (Variables|Default|GetSign)) (Utilities|Array|Get(acopy) (Variables|Default|GetBeforeLocationArray) _array_index) :!label _label_4))
                    (:NewEnumerator5
                      (goto _label_4))))))
            (:Finished
              (bind _cubearray (CallFunction|RebuildCubeArray))
              (Variables|Default|SetCubeArray _cubearray)
              (Utilities|FlowControl|Sequence
                (:then_0
                  (bind _bcorrect (CallFunction|IsCorrectFront)))
                (:then_1
                  (bind _bcorrect_2 (CallFunction|IsCorrectSide)))
                (:then_2
                  (if (and _bcorrect _bcorrect_2)
                    (Development|PrintString "Complete" true true "(R=0.000000,G=0.660000,B=1.000000,A=1.000000)" 1e+01)
                    (else
                      (Variables|Default|SetbRotating false)
                      (goto _label Reset))))))))))))

(event Input|KeyboardEvents|J
  (params (Key :type Key%20Structure :default "None"))
  (:Pressed
    (if (not (Variables|Default|GetbRotating))
      (Variables|Default|SetSign 1.0)
      (Utilities|FlowControl|DoOnce false :!label _label
        (:Completed
          (Variables|Default|SetbRotating true)
          (CallFunction|InitLocationArray)
          (bind _rotation (Timeline|タイムライン PlayFromStart)
            (:Update
              (for (_array_element _array_index) (Variables|Default|GetCubeArray)
                (if (Utilities|Array|ContainsItem (Variables|Default|GetSelectedIndexArray) _array_index)
                  (switch Utilities|FlowControl|Switch|SwitchonERotateType (Variables|Default|GetRotateType)
                    (:NewEnumerator0
                      (CallFunction|CubeRoll _array_element (* _rotation (Variables|Default|GetSign)) (Utilities|Array|Get(acopy) (Variables|Default|GetBeforeLocationArray) _array_index) :!label _label_2))
                    (:NewEnumerator1
                      (goto _label_2))
                    (:NewEnumerator2
                      (CallFunction|CubePitch _array_element (* _rotation (Variables|Default|GetSign)) (Utilities|Array|Get(acopy) (Variables|Default|GetBeforeLocationArray) _array_index) :!label _label_3))
                    (:NewEnumerator3
                      (goto _label_3))
                    (:NewEnumerator4
                      (CallFunction|CubeYaw _array_element (* _rotation (Variables|Default|GetSign)) (Utilities|Array|Get(acopy) (Variables|Default|GetBeforeLocationArray) _array_index) :!label _label_4))
                    (:NewEnumerator5
                      (goto _label_4))))))
            (:Finished
              (bind _cubearray (CallFunction|RebuildCubeArray))
              (Variables|Default|SetCubeArray _cubearray)
              (Utilities|FlowControl|Sequence
                (:then_0
                  (bind _bcorrect (CallFunction|IsCorrectFront)))
                (:then_1
                  (bind _bcorrect_2 (CallFunction|IsCorrectSide)))
                (:then_2
                  (if (and _bcorrect _bcorrect_2)
                    (Development|PrintString "Complete" true true "(R=0.000000,G=0.660000,B=1.000000,A=1.000000)" 1e+01)
                    (else
                      (Variables|Default|SetbRotating false)
                      (goto _label Reset))))))))))))

(event Input|KeyboardEvents|W
  (params (Key :type Key%20Structure :default "None"))
  ;[1 1 1] 入力から選択箇所を変更
  (:Pressed
    (if (not (Variables|Default|GetbRotating))
      (Variables|Default|SetRotateType "NewEnumerator2")
      (bind _selectionindexarray (CallFunction|CreateSelectionIndexArray (Variables|Default|GetRotateType)))
      (bind _output_get (Variables|Default|SetSelectedIndexArray _selectionindexarray))
      (CallFunction|ChangeCubeColor _output_get))))

(event Input|KeyboardEvents|S
  (params (Key :type Key%20Structure :default "None"))
  ;[1 1 1] 入力から選択箇所を変更
  (:Pressed
    (if (not (Variables|Default|GetbRotating))
      (Variables|Default|SetRotateType "NewEnumerator3")
      (bind _selectionindexarray (CallFunction|CreateSelectionIndexArray (Variables|Default|GetRotateType)))
      (bind _output_get (Variables|Default|SetSelectedIndexArray _selectionindexarray))
      (CallFunction|ChangeCubeColor _output_get))))

(fn ConstructionScript)

(fn CubeRoll
  (params (Cube :type Static%20Mesh%20Component%20Object%20Reference) (Rotation :type Float%20%28double-precision%29) (BeforeLocation :type Vector))
  (Transformation|SetRelativeTransform Cube (Math|Transform|ComposeTransforms (Math|Transform|MakeTransform (Math|Vector|MakeVector (.x BeforeLocation) (.y BeforeLocation) (.z BeforeLocation))) (Math|Transform|MakeTransform "0, 0, 0" (Math|Rotator|MakeRotator Rotation 0.0 0.0))) false false))

(fn CubePitch
  (params (Cube :type Static%20Mesh%20Component%20Object%20Reference) (Rotation :type Float%20%28double-precision%29) (BeforeLocation :type Vector))
  (Transformation|SetRelativeTransform Cube (Math|Transform|ComposeTransforms (Math|Transform|MakeTransform (Math|Vector|MakeVector (.x BeforeLocation) (.y BeforeLocation) (.z BeforeLocation))) (Math|Transform|MakeTransform "0, 0, 0" (Math|Rotator|MakeRotator 0.0 Rotation 0.0))) false false))

(fn CubeYaw
  (params (Cube :type Static%20Mesh%20Component%20Object%20Reference) (Rotation :type Float%20%28double-precision%29) (BeforeLocation :type Vector))
  (Transformation|SetRelativeTransform Cube (Math|Transform|ComposeTransforms (Math|Transform|MakeTransform (Math|Vector|MakeVector (.x BeforeLocation) (.y BeforeLocation) (.z BeforeLocation))) (Math|Transform|MakeTransform "0, 0, 0" (Math|Rotator|MakeRotator 0.0 0.0 Rotation))) false false))

(fn LoadSideAnswer
  (bind _returnvalue (Utilities|GetDataTableRow "/Game/CubePuzzle/AnswerData/T_Answer.T_Answer" "Stage1")
    (:then
      (for (_array_element _array_index) (.Side (Utilities|Struct|BreakST_table _returnvalue))
        (for _array_element_2 (Components|GetChildrenComponents (Variables|Default|GetDefaultSceneRoot) false)
          (if (Utilities|Enum|Equal(Enum) (Utilities|GetObjectName _array_element_2) (Utilities|String|Append "AnswerSidePanel" (Utilities|String|ToString(Integer) _array_index)))
            (bind _asstatic_mesh_component (Utilities|Casting|CastToStaticMeshComponent _array_element_2))
            (if _array_element
              (Rendering|Material|SetMaterial _asstatic_mesh_component 0 "/Game/CubePuzzle/Material/M_CubeExist.M_CubeExist")
              (else
                (Rendering|Material|SetMaterial _asstatic_mesh_component 0 "/Game/CubePuzzle/Material/M_CubeNone.M_CubeNone")))
            (Utilities|Array|Add (Variables|Default|GetSideAnswerPlateArray) _asstatic_mesh_component)))))))

(fn LoadFrontAnswer
  (bind _returnvalue (Utilities|GetDataTableRow "/Game/CubePuzzle/AnswerData/T_Answer.T_Answer" "Stage1")
    (:then
      (for (_array_element _array_index) (.Front (Utilities|Struct|BreakST_table _returnvalue))
        (for _array_element_2 (Components|GetChildrenComponents (Variables|Default|GetDefaultSceneRoot) false)
          (if (Utilities|Enum|Equal(Enum) (Utilities|GetObjectName _array_element_2) (Utilities|String|Append "AnswerFrontPanel" (Utilities|String|ToString(Integer) _array_index)))
            (bind _asstatic_mesh_component (Utilities|Casting|CastToStaticMeshComponent _array_element_2))
            (if _array_element
              (Rendering|Material|SetMaterial _asstatic_mesh_component 0 "/Game/CubePuzzle/Material/M_CubeExist.M_CubeExist")
              (else
                (Rendering|Material|SetMaterial _asstatic_mesh_component 0 "/Game/CubePuzzle/Material/M_CubeNone.M_CubeNone")))
            (Utilities|Array|Add (Variables|Default|GetFrontAnswerPlateArray) _asstatic_mesh_component)))))))

(fn LoadCube
  (bind _returnvalue (Utilities|GetDataTableRow "/Game/CubePuzzle/AnswerData/T_Answer.T_Answer" "Stage1")
    (:then
      (Variables|Default|SetbCubeExistArray (.Cube (Utilities|Struct|BreakST_table _returnvalue)))
      (for (_array_element _array_index) (.Cube (Utilities|Struct|BreakST_table _returnvalue))
        (for _array_element_2 (Components|GetChildrenComponents (Variables|Default|GetDefaultSceneRoot) false)
          (if (Utilities|Enum|Equal(Enum) (Utilities|GetObjectName _array_element_2) (Utilities|String|Append "Cube" (Utilities|String|ToString(Integer) _array_index)))
            (bind _asstatic_mesh_component (Utilities|Casting|CastToStaticMeshComponent _array_element_2))
            (if _array_element
              (Rendering|Material|SetMaterial _asstatic_mesh_component 0 "/Game/CubePuzzle/Material/M_CubeExist.M_CubeExist")
              ;[1 1 1] Cubeの有無をタグ付け
              (Variables|/Script/Engine.ActorComponent|SetComponentTags _asstatic_mesh_component (LocalVariables|GetExistTags))
              (else
                (Rendering|Material|SetMaterial _asstatic_mesh_component 0 "/Game/CubePuzzle/Material/M_CubeNone.M_CubeNone")
                (Variables|/Script/Engine.ActorComponent|SetComponentTags _asstatic_mesh_component (LocalVariables|GetEmptyTags))))
            (Utilities|Array|Add (Variables|Default|GetCubeArray) _asstatic_mesh_component)))))))

(fn InitLocationArray
  (Utilities|Array|Clear (Variables|Default|GetBeforeLocationArray))
  (for _array_element (Variables|Default|GetCubeArray)
    (Utilities|Array|Add (Variables|Default|GetBeforeLocationArray) (Variables|/Script/Engine.SceneComponent|GetRelativeLocation _array_element))))

(fn CreateSelectionIndexArray
  (params (RotateType :type ERotateType%20Enum :default "NewEnumerator0"))
  (bind _selectionarray (Variables|Default|GetSelectionArray))
  (switch Utilities|FlowControl|Switch|SwitchonERotateType RotateType
    (:NewEnumerator0
      (LocalVariables|SetReturnArray (.rolla _selectionarray)))
    (:NewEnumerator1
      (LocalVariables|SetReturnArray (.rollb _selectionarray)))
    (:NewEnumerator2
      (LocalVariables|SetReturnArray (.pitcha _selectionarray)))
    (:NewEnumerator3
      (LocalVariables|SetReturnArray (.pitchb _selectionarray)))
    (:NewEnumerator4
      (LocalVariables|SetReturnArray (.yawa _selectionarray)))
    (:NewEnumerator5
      (LocalVariables|SetReturnArray (.yawb _selectionarray))))
  (return (LocalVariables|GetReturnArray)))

(fn RebuildCubeArray
  (for _array_element (Variables|Default|GetCubeArray)
    (if (> (.x (Variables|/Script/Engine.SceneComponent|GetRelativeLocation _array_element)) 0.0)
      (if (> (.y (Variables|/Script/Engine.SceneComponent|GetRelativeLocation _array_element)) 0.0)
        (if (> (.z (Variables|/Script/Engine.SceneComponent|GetRelativeLocation _array_element)) 0.0)
          (LocalVariables|SetMoveToIndex 1)
          (else
            (LocalVariables|SetMoveToIndex 3)))
        (elif (> (.z (Variables|/Script/Engine.SceneComponent|GetRelativeLocation _array_element)) 0.0)
          (LocalVariables|SetMoveToIndex 5)
          (else
            (LocalVariables|SetMoveToIndex 7))))
      (elif (> (.y (Variables|/Script/Engine.SceneComponent|GetRelativeLocation _array_element)) 0.0)
        (if (> (.z (Variables|/Script/Engine.SceneComponent|GetRelativeLocation _array_element)) 0.0)
          (LocalVariables|SetMoveToIndex 0)
          (else
            (LocalVariables|SetMoveToIndex 2)))
        (elif (> (.z (Variables|/Script/Engine.SceneComponent|GetRelativeLocation _array_element)) 0.0)
          (LocalVariables|SetMoveToIndex 4)
          (else
            (LocalVariables|SetMoveToIndex 6)))))
    (Utilities|Array|SetArrayElem (LocalVariables|GetReturnArray) (LocalVariables|GetMoveToIndex) _array_element))
  (return (LocalVariables|GetReturnArray)))

(fn ChangeCubeColor
  (params (SelectionIndexArray :type Array%20of%20Integers))
  (for (_array_element _array_index) (Variables|Default|GetCubeArray)
    (if (Utilities|Array|ContainsItem SelectionIndexArray _array_index)
      (if (Components|ComponentHasTag _array_element "Exist")
        (Rendering|Material|SetMaterial _array_element 0 "/Game/CubePuzzle/Material/M_CubeSelectedExist.M_CubeSelectedExist")
        (else
          (Rendering|Material|SetMaterial _array_element 0 "/Game/CubePuzzle/Material/M_CubeSelectedNone.M_CubeSelectedNone")))
      (elif (Components|ComponentHasTag _array_element "Exist")
        (Rendering|Material|SetMaterial _array_element 0 "/Game/CubePuzzle/Material/M_CubeExist.M_CubeExist")
        (else
          (Rendering|Material|SetMaterial _array_element 0 "/Game/CubePuzzle/Material/M_CubeNone.M_CubeNone"))))))

(fn IsCorrectFront
  (bind _cubearray (Variables|Default|GetCubeArray))
  (bind _cubearray_2 (Variables|Default|GetCubeArray))
  (bind _bcorrectarray (LocalVariables|GetbCorrectArray))
  (bind _returnvalue (Utilities|GetDataTableRow "/Game/CubePuzzle/AnswerData/T_Answer.T_Answer" "Stage1")
    (:then
      (for (_array_element _array_index) (.Front (Utilities|Struct|BreakST_table _returnvalue))
        (switch int _array_index
          (:0
            (LocalVariables|SetHandleIndex1 0)
            (LocalVariables|SetHandleIndex2 1)
            (if _array_element
              (Utilities|Array|Add _bcorrectarray (or (Components|ComponentHasTag (Utilities|Array|Get(acopy) _cubearray_2 (LocalVariables|GetHandleIndex1)) "Exist") (Components|ComponentHasTag (Utilities|Array|Get(acopy) _cubearray_2 (LocalVariables|GetHandleIndex2)) "Exist")) :!label _label)
              (else
                (Utilities|Array|Add _bcorrectarray (and (Components|ComponentHasTag (Utilities|Array|Get(acopy) _cubearray (LocalVariables|GetHandleIndex1)) "Empty") (Components|ComponentHasTag (Utilities|Array|Get(acopy) _cubearray (LocalVariables|GetHandleIndex2)) "Empty")) :!label _label_2))))
          (:1
            (LocalVariables|SetHandleIndex1 4)
            (LocalVariables|SetHandleIndex2 5)
            (if _array_element
              (goto _label)
              (else
                (goto _label_2))))
          (:2
            (LocalVariables|SetHandleIndex1 2)
            (LocalVariables|SetHandleIndex2 3)
            (if _array_element
              (goto _label)
              (else
                (goto _label_2))))
          (:3
            (LocalVariables|SetHandleIndex1 6)
            (LocalVariables|SetHandleIndex2 7)
            (if _array_element
              (goto _label)
              (else
                (goto _label_2))))))
      (return (not (Utilities|Array|ContainsItem (LocalVariables|GetbCorrectArray) false))))))

(fn IsCorrectSide
  (bind _cubearray (Variables|Default|GetCubeArray))
  (bind _cubearray_2 (Variables|Default|GetCubeArray))
  (bind _bcorrectarray (LocalVariables|GetbCorrectArray))
  (bind _returnvalue (Utilities|GetDataTableRow "/Game/CubePuzzle/AnswerData/T_Answer.T_Answer" "Stage1")
    (:then
      (for (_array_element _array_index) (.Side (Utilities|Struct|BreakST_table _returnvalue))
        (switch int _array_index
          (:0
            (LocalVariables|SetHandleIndex1 0)
            (LocalVariables|SetHandleIndex2 4)
            (if _array_element
              (Utilities|Array|Add _bcorrectarray (or (Components|ComponentHasTag (Utilities|Array|Get(acopy) _cubearray_2 (LocalVariables|GetHandleIndex1)) "Exist") (Components|ComponentHasTag (Utilities|Array|Get(acopy) _cubearray_2 (LocalVariables|GetHandleIndex2)) "Exist")) :!label _label)
              (else
                (Utilities|Array|Add _bcorrectarray (and (Components|ComponentHasTag (Utilities|Array|Get(acopy) _cubearray (LocalVariables|GetHandleIndex1)) "Empty") (Components|ComponentHasTag (Utilities|Array|Get(acopy) _cubearray (LocalVariables|GetHandleIndex2)) "Empty")) :!label _label_2))))
          (:1
            (LocalVariables|SetHandleIndex1 1)
            (LocalVariables|SetHandleIndex2 5)
            (if _array_element
              (goto _label)
              (else
                (goto _label_2))))
          (:2
            (LocalVariables|SetHandleIndex1 2)
            (LocalVariables|SetHandleIndex2 6)
            (if _array_element
              (goto _label)
              (else
                (goto _label_2))))
          (:3
            (LocalVariables|SetHandleIndex1 3)
            (LocalVariables|SetHandleIndex2 7)
            (if _array_element
              (goto _label)
              (else
                (goto _label_2))))))
      (return (not (Utilities|Array|ContainsItem (LocalVariables|GetbCorrectArray) false))))))